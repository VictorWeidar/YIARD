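; BP_Gate is an enemy spawner that releases BP_EnemyCharger actors at its Spawnpoint transform.
; Tick calls SpawnEnemy every frame, relying on Delay ignoring re-triggers while pending to pace spawns at random 2–5 second intervals.
; A counter allows spawns while SpawnedEnemies is at or below AmountOfEnemies, then each later delay completion just prints "DONE".
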(event `self.ReceiveTick`
  (params (DeltaSeconds :type "Float (single-precision)"))
  (`self.SpawnEnemy`))

(event `SpawnEnemy`
  (`KismetSystemLibrary.Delay` (`KismetMathLibrary.RandomFloatInRange` 2.0 5.0))
  (if (<= (`self.Spawned Enemies`) (`self.AmountOfEnemies`))
    (`|SpawnActorFromClass` "/Game/Blueprints/BP_EnemyCharger.BP_EnemyCharger_C" (`SceneComponent.K2_GetComponentToWorld` (`self.Spawnpoint`)) "Undefined" "OverrideRootScale" null null)
    (set `self.Spawned Enemies` (+ (`self.Spawned Enemies`) 1.0))
    (else
      (`KismetSystemLibrary.PrintString` "DONE"))))

(fn `UserConstructionScript`)