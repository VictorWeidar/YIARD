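; Pumpkin monster enemy that runs BT_Pumpkin and, a second after seeing the player, moves to them, setting its run animation once the move finishes.
; TakeDamage drains health; death bursts the head with a splat, ragdolls the mesh and destroys the actor after five seconds.
; A box overlap tracks PlayerInRange.
; DealDamage subtracts player Health and re-calls itself immediately while any remains.
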(event `self.PawnSensing.OnSeePawn`
  (params (Pawn :type "Pawn Object Reference"))
  ;[1 1 1] Wait for detect anim to finish
  (`KismetSystemLibrary.Delay` 1.0)
  (bind _asfps_controller (cast `/Game/Blueprints/FPS_Controller` Pawn))
  (`|AIMoveTo` self (0.0 0.0 0.0) _asfps_controller
    (:`then`
      ;[1 1 1] Enable Run Anim
      (bind _asabp_pumpkin (cast `/Game/Characters/Monsters/Pumpkin/Animations/ABP_Pumpkin` (`SkeletalMeshComponent.GetAnimInstance` (`self.Mesh`))))
      (set `/Game/Characters/Monsters/Pumpkin/Animations/ABP_Pumpkin.IsRunning` true _asabp_pumpkin))))

(event `TakeDamage`
  (params (DamagePercentage :type "Float (double-precision)"))
  (bind _mesh (`self.Mesh`))
  (bind _head (`self.Head`))
  ;[1 1 1] Take damage + Death Sequence
  (bind _output_get (set `self.PumpkinHealth` (- (`self.PumpkinHealth`) DamagePercentage)))
  (if (<= _output_get 0.0)
    (`GameplayStatics.SpawnEmitterAtLocation` "/Game/Particles/P_PumpkinSplat.P_PumpkinSplat" (`SceneComponent.K2_GetComponentLocation` _head))
    (`ActorComponent.K2_DestroyComponent` _head)
    (`ActorComponent.K2_DestroyComponent` (`self.Collision`))
    (`PrimitiveComponent.SetSimulatePhysics` _mesh true)
    (bind _asabp_pumpkin (cast `/Game/Characters/Monsters/Pumpkin/Animations/ABP_Pumpkin` (`SkeletalMeshComponent.GetAnimInstance` _mesh)))
    (set `/Game/Characters/Monsters/Pumpkin/Animations/ABP_Pumpkin.IsDead` true _asabp_pumpkin)
    (`KismetSystemLibrary.Delay` 5.0)
    (`self.K2_DestroyActor`)))

(event `self.Box.OnComponentBeginOverlap`
  (params (OverlappedComponent :type "PrimitiveComponent Object Reference") (OtherActor :type "Actor Object Reference") (OtherComp :type "PrimitiveComponent Object Reference") (OtherBodyIndex :type Integer) (bFromSweep :type Boolean) (SweepResult :type "HitResult Structure (by ref)"))
  ;[1 1 1] Hitting player
  (cast `/Game/Blueprints/FPS_Controller` OtherActor)
  (set `self.PlayerInRange` true)
  (`KismetSystemLibrary.PrintString` "In range"))

(event `self.ReceiveBeginPlay`
  ;[1 1 1] Switch for Patrol State
  (`AIController.RunBehaviorTree` (`AIBlueprintHelperLibrary.GetAIController` self) "/Game/Characters/Monsters/Pumpkin/AI/BT_Pumpkin.BT_Pumpkin"))

(event `self.Box.OnComponentEndOverlap`
  (params (OverlappedComponent :type "PrimitiveComponent Object Reference") (OtherActor :type "Actor Object Reference") (OtherComp :type "PrimitiveComponent Object Reference") (OtherBodyIndex :type Integer))
  ;[1 1 1] Hitting player
  (cast `/Game/Blueprints/FPS_Controller` OtherActor)
  (set `self.PlayerInRange` false)
  (`KismetSystemLibrary.PrintString` "Not In Range"))

(event `DealDamage`
  ;[1 1 1] Hitting player
  (bind _asfps_controller (cast `/Game/Blueprints/FPS_Controller` (`GameplayStatics.GetPlayerCharacter` 0)))
  (bind _output_get (set `/Game/Blueprints/FPS_Controller.Health` (- (`/Game/Blueprints/FPS_Controller.Health` _asfps_controller) (`self.PumpkinDamage`)) _asfps_controller))
  (if (<= _output_get 0.0)
    (`KismetSystemLibrary.PrintString` "DEAD")
    (else
      (`self.DealDamage`)
      (`KismetSystemLibrary.PrintString` "Smack")
      (set `self.HasAttacked` true))))

(fn `UserConstructionScript`)